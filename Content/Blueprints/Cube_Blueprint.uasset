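; Shootable shape actor that cycles its static mesh through a Shapes array on BeginPlay and on every hit.
; Each change wraps the index, swaps the material and sets IsCube according to whether the new mesh is SM_Cube.
; BeginPlay shares the hit logic, using a Created flag to skip scoring-style side effects on the first pass.
; Later hits notify BP_FirstPersonGameMode, then destroy the other actor if it is a BP_FirstPersonProjectile.
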(event EventBeginPlay
  (bind _shapes (Variables|Default|GetShapes))
  (bind _staticmeshcomponent (Variables|Debug|GetStaticMeshComponent))
  ;[0.15 0.15 0.15 0.5] Set Initial Shape
  (Components|StaticMesh|SetStaticMesh (Variables|Debug|GetStaticMeshComponent) (Utilities|Array|Get(acopy) (Variables|Default|GetShapes) (Variables|Default|GetShapeIncrement)))
  ;[1 1 1] Toggle between shapes in the array after hitting the object. If object is a SM_Cube then set Is Cube to True
  (bind _output_get (Variables|Default|SetShapeIncrement (+ (Variables|Default|GetShapeIncrement) 1)))
  (if (== (Utilities|Array|Length _shapes) (Variables|Default|GetShapeIncrement))
    (Variables|Default|SetShapeIncrement 0))
  (Components|StaticMesh|SetStaticMesh (Variables|Debug|GetStaticMeshComponent) (Utilities|Array|Get(acopy) _shapes _output_get))
  (if (== (Utilities|Array|Get(acopy) _shapes _output_get) "/Game/LevelPrototyping/Meshes/SM_Cube.SM_Cube")
    (Rendering|Material|SetMaterial _staticmeshcomponent 0 "/Engine/MapTemplates/Materials/BasicAsset03.BasicAsset03")
    (Variables|Default|SetIsCube true)
    (else
      (Rendering|Material|SetMaterial _staticmeshcomponent 0 "/Engine/VREditor/BasicMeshes/MI_Cube_03.MI_Cube_03")
      (Variables|Default|SetIsCube false)))
  (if (Variables|Default|GetCreated)
    (bind _asbp_first_person_game_mode (Utilities|Casting|CastToBP_FirstPersonGameMode (Game|GetGameMode)))
    (Default|OnCubeHitHandlerEvent _asbp_first_person_game_mode)
    (bind _asbp_first_person_projectile (Utilities|Casting|CastToBP_FirstPersonProjectile (stale Collision|EventHit Other)))
    (Actor|DestroyActor _asbp_first_person_projectile)
    (else
      (Variables|Default|SetCreated true))))

(event Collision|EventHit
  (params (MyComp :type Primitive%20Component%20Object%20Reference) (Other :type Actor%20Object%20Reference) (OtherComp :type Primitive%20Component%20Object%20Reference) (bSelfMoved :type Boolean) (HitLocation :type Vector :default "0, 0, 0") (HitNormal :type Vector :default "0, 0, 0") (NormalImpulse :type Vector :default "0, 0, 0") (Hit :type Hit%20Result%20Structure%20%28by%20ref%29))
  (bind _shapes (Variables|Default|GetShapes))
  (bind _staticmeshcomponent (Variables|Debug|GetStaticMeshComponent))
  ;[1 1 1] Toggle between shapes in the array after hitting the object. If object is a SM_Cube then set Is Cube to True
  (bind _output_get (Variables|Default|SetShapeIncrement (+ (Variables|Default|GetShapeIncrement) 1)))
  (if (== (Utilities|Array|Length _shapes) (Variables|Default|GetShapeIncrement))
    (Variables|Default|SetShapeIncrement 0))
  (Components|StaticMesh|SetStaticMesh (Variables|Debug|GetStaticMeshComponent) (Utilities|Array|Get(acopy) _shapes _output_get))
  (if (== (Utilities|Array|Get(acopy) _shapes _output_get) "/Game/LevelPrototyping/Meshes/SM_Cube.SM_Cube")
    (Rendering|Material|SetMaterial _staticmeshcomponent 0 "/Engine/MapTemplates/Materials/BasicAsset03.BasicAsset03")
    (Variables|Default|SetIsCube true)
    (else
      (Rendering|Material|SetMaterial _staticmeshcomponent 0 "/Engine/VREditor/BasicMeshes/MI_Cube_03.MI_Cube_03")
      (Variables|Default|SetIsCube false)))
  (if (Variables|Default|GetCreated)
    (bind _asbp_first_person_game_mode (Utilities|Casting|CastToBP_FirstPersonGameMode (Game|GetGameMode)))
    (Default|OnCubeHitHandlerEvent _asbp_first_person_game_mode)
    (bind _asbp_first_person_projectile (Utilities|Casting|CastToBP_FirstPersonProjectile Other))
    (Actor|DestroyActor _asbp_first_person_projectile)
    (else
      (Variables|Default|SetCreated true))))

(fn ConstructionScript)