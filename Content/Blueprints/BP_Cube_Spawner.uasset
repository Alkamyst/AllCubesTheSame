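; BP_Cube_Spawner is an actor that scatters randomized Cube_Blueprint instances around its location when play begins.
; It reads the spawn count from CubeNum on the GI_Main game instance and does nothing if that cast fails.
; Each spawn gets a random offset within a box longest in X and narrowest in Y, a random rotation, and a random ShapeIncrement from three possible values.
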(event EventBeginPlay
  (bind _returnvalue (Transformation|GetActorLocation))
  (bind _asgi_main (Utilities|Casting|CastToGI_Main (Game|GetGameInstance)))
  (for _index (range 1 (Variables|/Game/Blueprints/GI_Main.GI_Main_C|GetCubeNum _asgi_main))
    (Game|SpawnActorfromClass "/Game/Blueprints/Cube_Blueprint.Cube_Blueprint_C" (Math|Transform|MakeTransform (Math|Vector|MakeVector (+ (Math|Random|RandomFloatinRange -1e+03 1e+03) (.x _returnvalue)) (+ (Math|Random|RandomFloatinRange -1e+02 1e+02) (.y _returnvalue)) (+ (Math|Random|RandomFloatinRange -4e+02 4e+02) (.z _returnvalue))) (Math|Rotator|MakeRotator (Math|Random|RandomFloatinRange 0.0 3.6e+02) (Math|Random|RandomFloatinRange 0.0 3.6e+02) (Math|Random|RandomFloatinRange 0.0 3.6e+02)) "1.000000,1.000000,1.000000") "Undefined" "MultiplyWithRoot" 0 0 (Math|Random|RandomIntegerinRange 0 2) false 0)))

(fn ConstructionScript)